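; BP_Enemy is an enemy actor that follows the level's BP_SplinePath at its Speed.
; BeginPlay caches the spline and BP_EnemySpawner; Tick advances distance along the spline, setting location and rotation.
; TakeDamage sets Health to Damage minus Health (operands reversed) and calls Die at zero or below.
; Death and reaching the end both decrement the spawner's count and destroy the actor; the TDGamemode damage call is unconnected.
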(event EventBeginPlay
  (bind _returnvalue (Actor|GetActorOfClass "/Game/Enemy/EnemyPath/BP_SplinePath.BP_SplinePath_C"))
  (Variables|Default|SetSplineRef _returnvalue)
  (bind _returnvalue_2 (Actor|GetActorOfClass "/Game/Enemy/EnemySpawner/BP_EnemySpawner.BP_EnemySpawner_C"))
  (Variables|Default|SetSpawnerRef _returnvalue_2))

(event EventTick
  (params (DeltaSeconds :type Float%20%28single-precision%29))
  (CallFunction|MoveAlongSpline DeltaSeconds))

(fn ConstructionScript)

(fn TakeDamage
  (params (Damage :type Float%20%28double-precision%29))
  (bind _output_get (Variables|Default|SetHealth (- Damage (Variables|Default|GetHealth))))
  (if (<= _output_get 0.0)
    (CallFunction|Die)))

(fn Die
  (Default|DecreaseEnemyCount (Variables|Default|GetSpawnerRef))
  (Actor|DestroyActor))

(fn MoveAlongSpline
  (params (A :type Float%20%28double-precision%29))
  (bind _splineref (Variables|Default|GetSplineRef))
  (bind _spline (Variables|/Game/Enemy/EnemyPath/BP_SplinePath.BP_SplinePath_C|GetSpline _splineref))
  (bind _output_get (Variables|Default|SetDistanceAlongSpline (+ (* A (Variables|Default|GetSpeed)) (Variables|Default|GetDistanceAlongSpline))))
  (Transformation|SetActorTransform (Math|Transform|MakeTransform (Spline|GetLocationatDistanceAlongSpline _spline _output_get "World") (Spline|GetRotationatDistanceAlongSpline _spline _output_get "World") "1.000000,1.000000,1.000000"))
  (if (>= (Variables|Default|GetDistanceAlongSpline) (Spline|GetSplineLength (Variables|/Game/Enemy/EnemyPath/BP_SplinePath.BP_SplinePath_C|GetSpline (Variables|Default|GetSplineRef))))
    (CallFunction|ReachedEnd)))

(fn ReachedEnd
  (Default|DecreaseEnemyCount (Variables|Default|GetSpawnerRef))
  (Actor|DestroyActor))