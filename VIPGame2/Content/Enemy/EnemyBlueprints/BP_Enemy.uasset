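; Tower defense enemy that follows the BP_SplinePath spline each tick and damages TDGameModeBase upon reaching the end.
; Death or arrival decrements the BP_EnemySpawner count; dead enemies stop and are destroyed after a delay.
; Slow, burn and toxic respect immunities and use named-function timers, with burn re-arming itself per damage tick.
; Toxic deals only one tick because its elapsed time jumps past the duration, and stun only sets an unread flag.
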(event EventBeginPlay
  (bind _returnvalue (Actor|GetActorOfClass "/Game/Enemy/EnemyPath/BP_SplinePath.BP_SplinePath_C"))
  (Variables|Movement|SetSplineRef _returnvalue)
  (bind _returnvalue_2 (Actor|GetActorOfClass "/Game/Enemy/EnemySpawner/BP_EnemySpawner.BP_EnemySpawner_C"))
  (Variables|Spawning|SetSpawnerRef _returnvalue_2))

(event EventTick
  (params (DeltaSeconds :type Float%20%28single-precision%29))
  (CallFunction|MoveAlongSpline DeltaSeconds))

(fn ConstructionScript)

(fn TakeDamage
  (params (Damage :type Float%20%28double-precision%29))
  (if (not (Variables|Default|GetisDead))
    (bind _output_get (Variables|Default|SetHealth (- (Variables|Default|GetHealth) Damage)))
    (if (<= _output_get 0.0)
      (Development|PrintString "Died")
      (CallFunction|Die))))

(fn Die
  (Default|DecreaseEnemyCount (Variables|Spawning|GetSpawnerRef))
  (Variables|Default|SetisDead true)
  (Utilities|Time|SetTimerbyFunctionName 0 "DestroySelf" 5.0))

(fn MoveAlongSpline
  (params (A :type Float%20%28double-precision%29))
  (bind _splineref (Variables|Movement|GetSplineRef))
  (bind _spline (Variables|/Game/Enemy/EnemyPath/BP_SplinePath.BP_SplinePath_C|GetSpline _splineref))
  (if (not (Variables|Default|GetisDead))
    (bind _output_get (Variables|Movement|SetDistanceAlongSpline (+ (* A (* (Variables|Effects|GetslowModifier) (Variables|Movement|GetSpeed))) (Variables|Movement|GetDistanceAlongSpline))))
    (Transformation|SetActorTransform (Math|Transform|MakeTransform (Spline|GetLocationatDistanceAlongSpline _spline _output_get "World") (Spline|GetRotationatDistanceAlongSpline _spline _output_get "World") "1.000000,1.000000,1.000000"))
    (if (>= (Variables|Movement|GetDistanceAlongSpline) (Spline|GetSplineLength (Variables|/Game/Enemy/EnemyPath/BP_SplinePath.BP_SplinePath_C|GetSpline (Variables|Movement|GetSplineRef))))
      (CallFunction|ReachedEnd))))

(fn ReachedEnd
  (Default|DecreaseEnemyCount (Variables|Spawning|GetSpawnerRef))
  (bind _astdgame_mode_base (Utilities|Casting|CastToTDGameModeBase (Game|GetGameMode))
    (:then
      (Default|TakeDamage _astdgame_mode_base (Variables|Default|GetDamage))
      (Actor|DestroyActor))
    (:CastFailed
      (Development|PrintString "cast failed"))))

(fn GetSlowed
  (params (SlowDuration :type Float%20%28double-precision%29) (slowAmount :type Float%20%28double-precision%29))
  (if (not (Variables|Immunities|GetslowImmunity))
    (Variables|Effects|SetslowModifier (- 1.0 slowAmount))
    (Utilities|Time|SetTimerbyFunctionName 0 "StopSlowEffect" SlowDuration)))

(fn StopSlowEffect
  (Variables|Effects|SetslowModifier 1.0))

(fn Burn
  (bind _burnticktime (Variables|Fire|GetburnTickTime))
  (if (>= (Variables|Fire|Gettimeburning) (Variables|Fire|GetburnTime))
    (Development|PrintString "Finnished burning")
    (Variables|Fire|SetIsBurning false)
    (else
      (CallFunction|TakeDamage (Variables|Fire|GetburnDamage))
      (Variables|Fire|Settimeburning (+ (Variables|Fire|Gettimeburning) _burnticktime))
      (Utilities|Time|SetTimerbyFunctionName 0 "Burn" _burnticktime))))

(fn StartBurning
  (params (burnDamage :type Float%20%28double-precision%29) (burnTime :type Float%20%28double-precision%29) (burnTickTime :type Float%20%28double-precision%29))
  (if (not (Variables|Immunities|GetburnImmunity))
    (Variables|Fire|SetburnDamage burnDamage)
    (Variables|Fire|SetburnTime burnTime)
    (Variables|Fire|SetburnTickTime burnTickTime)
    (Variables|Fire|Settimeburning 0.0)
    (Variables|Fire|SetIsBurning true)
    (CallFunction|Burn)))

(fn StartToxic
  (params (toxicTime :type Float%20%28double-precision%29) (toxicDamage :type Float%20%28double-precision%29) (toxicTickTime :type Float%20%28double-precision%29))
  (if (not (Variables|Immunities|GettoxicImmunity))
    (Variables|Toxic|SettoxicDuration toxicTime)
    (Variables|Toxic|SettoxicDamage toxicDamage)
    (Variables|Toxic|SettoxicTickTime toxicTickTime)
    (Variables|Toxic|SetIsAffectedByToxic true)
    (Variables|Toxic|SettimeAffectedByToxic 0.0)
    (CallFunction|Toxic)))

(fn Toxic
  (bind _toxicduration (Variables|Toxic|GettoxicDuration))
  (bind _toxicticktime (Variables|Toxic|GettoxicTickTime))
  (if (>= (Variables|Toxic|GettimeAffectedByToxic) _toxicduration)
    (Development|PrintString "Stop being affected by toxic")
    (Variables|Toxic|SetIsAffectedByToxic false)
    (else
      (CallFunction|TakeDamage (Variables|Toxic|GettoxicDamage))
      (Variables|Toxic|SettimeAffectedByToxic (+ _toxicduration _toxicticktime))
      (Utilities|Time|SetTimerbyFunctionName 0 "Toxic" _toxicticktime))))

(fn GetIsDead
  (return (Variables|Default|GetisDead)))

(fn DestroySelf
  (Actor|DestroyActor))

(fn GetStunned
  (Variables|Stun|SetisStunned true))

(fn StopStun
  (Variables|Stun|SetisStunned false))