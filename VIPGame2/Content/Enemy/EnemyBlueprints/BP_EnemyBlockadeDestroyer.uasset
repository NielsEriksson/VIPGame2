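; An enemy Blueprint that destroys a nearby blockade, sacrificing itself in the process.
; Each tick, after the parent Tick, it scans all Blockader actors and picks the first one found within Range, not necessarily the nearest.
; On a hit, it destroys both that blockade and itself; if none exist, it only prints a debug message.
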(event EventBeginPlay
  (|CallParentFunction) ; This node is disabled and will not be called.\nDrag off pins to build functionality.
)

(event Collision|EventActorBeginOverlap
  (params (OtherActor :type Actor%20Object%20Reference)))

(event EventTick
  (params (DeltaSeconds :type Float%20%28single-precision%29))
  (|CallParentFunction DeltaSeconds)
  (bind (_closeblockade _bool) (CallFunction|IsClosetoBlockade))
  (if _bool
    (CallFunction|DestroyBlockade _closeblockade)))

(fn ConstructionScript
  (|CallParentFunction))

(fn IsClosetoBlockade
  (bind _outactors (Actor|GetAllActorsOfClass "/Game/GameObjects/Objects/Blockader.Blockader_C"))
  (if (Utilities|Array|IsNotEmpty _outactors)
    (for _array_element _outactors
      (if (<= (Math|Vector|Distance(Vector) (Transformation|GetActorLocation _array_element) (Transformation|GetActorLocation)) (Variables|Default|Getrange))
        (return _array_element true)))
    (return 0 false)
    (else
      (Development|PrintString "no blockade exists"))))

(fn DestroyBlockade
  (params (blockade :type Blockader%20Object%20Reference))
  (Actor|DestroyActor blockade)
  (Actor|DestroyActor))