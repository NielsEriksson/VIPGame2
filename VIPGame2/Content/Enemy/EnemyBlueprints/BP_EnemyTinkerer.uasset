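; Tinkerer enemy Blueprint, apparently meant to disable nearby towers on a cooldown, though the disable effect is unfinished.
; While off cooldown, Tick gathers PlaceableBaseAsset actors within Range, picks the closest and calls DisableTower.
; DisableTower only starts the DisableCD timer that clears OnCooldown; its tower cast is unconnected.
; HasColsestTower is only ever set false here, so that cooldown branch never runs as written.
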(event EventBeginPlay
  (|CallParentFunction))

(event Collision|EventActorBeginOverlap
  (params (OtherActor :type Actor%20Object%20Reference)))

(event EventTick
  (params (DeltaSeconds :type Float%20%28single-precision%29))
  (|CallParentFunction DeltaSeconds)
  (if (not (Variables|Default|GetonCooldown))
    (CallFunction|FindTowersinRange)
    (CallFunction|FindClosestTower)
    (CallFunction|DisableTower)))

(fn ConstructionScript
  (|CallParentFunction))

(fn FindTowersinRange
  (Utilities|Array|Clear (Variables|Default|GettowersInRange))
  (bind _outactors (Actor|GetAllActorsOfClass "/Game/GameObjects/Objects/PlaceableBaseAsset.PlaceableBaseAsset_C"))
  (for _array_element _outactors
    (if (<= (Math|Vector|Distance(Vector) (Transformation|GetActorLocation _array_element) (Transformation|GetActorLocation)) (Variables|Default|GetRange))
      (Utilities|Array|Add (Variables|Default|GettowersInRange) _array_element))))

(fn FindClosestTower
  (bind _returnvalue (Transformation|GetActorLocation))
  (bind _towersinrange (Variables|Default|GettowersInRange))
  (if (Utilities|Array|IsEmpty _towersinrange)
    (Development|PrintString "array empty no tower in range")
    (Variables|Default|SethasColsestTower false)
    (else
      ;[1 1 1] Reset closest tower
      (Variables|Default|SetclosestTower (Utilities|Array|Get(acopy) _towersinrange))
      (Variables|Default|SethasColsestTower false)
      (for _array_element _towersinrange
        (if (< (Math|Vector|Distance(Vector) (Transformation|GetActorLocation _array_element) _returnvalue) (Math|Vector|Distance(Vector) _returnvalue (Transformation|GetActorLocation (Variables|Default|GetclosestTower))))
          (Variables|Default|SetclosestTower _array_element)))
      (Development|PrintString (Utilities|GetDisplayName (Variables|Default|GetclosestTower))))))

(fn DisableTower
  (if (Variables|Default|GethasColsestTower)
    (Variables|Default|SetonCooldown true)
    (Utilities|Time|SetTimerbyFunctionName 0 "CooldownDone" (Variables|Default|GetDisableCD))))

(fn CooldownDone
  (Variables|Default|SetonCooldown false))