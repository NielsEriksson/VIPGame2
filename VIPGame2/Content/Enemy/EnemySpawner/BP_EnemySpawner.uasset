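; Enemy spawner actor that spawns waves from a weight budget, starting the first wave shortly after BeginPlay.
; Every NWave waves the budget grows, and a repeating timer spawns random EnemyTypes at the spawner's transform, deducting each class-default Weight until none remains.
; Random picks retry until one fits, but EnemyFound is never reset.
; EnemyDied checks EnemiesAlive for zero without decrementing it, then only prints and delays, with no next-wave call.
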(event Custom|EnemyDied
  (Utilities|EnemyDie))

(event EventBeginPlay
  (Development|PrintString "Wait for round to start")
  (Utilities|FlowControl|Delay 5.0)
  (Development|PrintString "Done waiting")
  (CallFunction|StartWave))

(fn ConstructionScript)

(fn SpawnEnemy
  (bind _output (CallFunction|GetRandomEnemyType))
  (Game|SpawnActorfromClass (Utilities|Array|Get(acopy) (Variables|Default|GetEnemyTypes) _output) (Transformation|GetActorTransform) "Undefined" "MultiplyWithRoot" 0 0)
  (Math|Integer|IncrementInt (Variables|Default|GetenemiesAlive)
    (:%20%20
      (bind _output_get (Variables|Default|SetcurrentWeight (- (Variables|Default|GetcurrentWeight) (.Weight (Utilities|GetClassDefaults (Utilities|Array|Get(acopy) (Variables|Default|GetEnemyTypes) _output))))))
      (if (> _output_get 0)
        (Utilities|Time|SetTimerbyFunctionName 0 "SpawnEnemy" (Variables|Default|GettimeBetweenSpawn))))))

(fn GetRandomEnemyType
  (while (not (LocalVariables|GetEnemyFound))
    (bind _ouput (CallFunction|GetRandomIndex))
    (bind _output_get (LocalVariables|Setindex _ouput))
    (if (<= (.Weight (Utilities|GetClassDefaults (Utilities|Array|Get(acopy) (Variables|Default|GetEnemyTypes) _output_get))) (Variables|Default|GetcurrentWeight))
      (LocalVariables|SetEnemyFound true)
      (else
        (Development|PrintString "Couldnt find enemy to spawn"))))
  (return _output_get))

(fn StartWave
  (Development|PrintString "Starting next wave")
  (Math|Integer|IncrementInt (Variables|Default|GetCurrentWave)
    (:%20%20
      (CallFunction|IncreaseTotalWeight)
      (Variables|Default|SetcurrentWeight (Variables|Default|GettotalWeight))
      (CallFunction|SpawnEnemy))))

(fn GetRandomIndex
  (bind _output_get (LocalVariables|Setindex (Math|Random|RandomIntegerinRange 0 (- (Utilities|Array|Length (Variables|Default|GetEnemyTypes)) 1))))
  (return _output_get))

(fn IncreaseTotalWeight
  (if (== (Math|Integer|%(Integer) (Variables|Default|GetCurrentWave) (Variables|Default|GetNWave)) 0)
    (Variables|Default|SettotalWeight (+ (Variables|Default|GettotalWeight) (Variables|Default|GetWeightIncreasePerNWave)))
    (Development|PrintString "Total weight increased")))