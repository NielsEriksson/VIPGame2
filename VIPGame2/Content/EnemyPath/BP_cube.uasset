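; BP_cube is an actor that travels along a spline path in the level.
; On BeginPlay it finds the BP_SplinePath actor by class and stores it as its path reference.
; Each tick it advances a distance by Speed times delta time and sets its world location and rotation from the spline at that distance.
; The distance grows without any clamp, wrap or end-of-path handling.
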(event EventBeginPlay
  (bind _returnvalue (Actor|GetActorOfClass "/Game/EnemyPath/BP_SplinePath.BP_SplinePath_C"))
  (Variables|Default|SetSplineRef _returnvalue))

(event EventTick
  (params (DeltaSeconds :type Float%20%28single-precision%29))
  (bind _splineref (Variables|Default|GetSplineRef))
  (bind _spline (Variables|/Game/EnemyPath/BP_SplinePath.BP_SplinePath_C|GetSpline _splineref))
  (bind _output_get (Variables|Default|SetDistanceAlongSpline (+ (* DeltaSeconds (Variables|Default|GetSpeed)) (Variables|Default|GetDistanceAlongSpline))))
  (Transformation|SetActorTransform (Math|Transform|MakeTransform (Spline|GetLocationatDistanceAlongSpline _spline _output_get "World") (Spline|GetRotationatDistanceAlongSpline _spline _output_get "World") "1.000000,1.000000,1.000000")))

(fn ConstructionScript)